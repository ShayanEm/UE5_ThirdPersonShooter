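; Third-person player character with Enhanced Input movement, rifle equip, aiming and automatic fire, which also creates the HUD on BeginPlay.
; Equipping toggles a flag and, after a delay, rifle visibility; aiming switches to strafe rotation while a timeline pulls in the spring arm.
; Holding fire with the rifle equipped loops a timer playing a montage, whose notify triggers a camera line trace, impact and muzzle effects, shake and sound.
; The trace applies no damage.
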(event Custom|Fire%20Rifle
  (bind _camera (Variables|Default|GetCamera))
  (bind _rifle (Variables|Default|GetRifle))
  (bind _returnvalue (Transformation|GetSocketTransform _rifle "Muzzle" "RTS_World"))
  (bind _returnvalue_2 (Transformation|GetWorldLocation _camera))
  (Animation|Montage|PlayMontage (Variables|Character|GetMesh) "/Game/Characters/Animations/Rifle/Fire_Rifle_Montage.Fire_Rifle_Montage"
    (:OnNotifyBegin
      (Utilities|FlowControl|Sequence
        (:then_0
          (bind (_outhit _returnvalue_3) (Collision|LineTraceByChannel _returnvalue_2 (+ _returnvalue_2 (* (Math|Vector|GetForwardVector (Transformation|GetWorldRotation _camera)) 5e+03)) "TraceTypeQuery1" false 0 "ForDuration"))
          (if _returnvalue_3
            (Effects|SpawnEmitteratLocation "/Game/InfinityBladeEffects/Effects/FX_Monsters/FX_Monster_Troll/death/P_TrollDeathImpact.P_TrollDeathImpact" (.ImpactPoint (Collision|BreakHitResult _outhit)) (Math|Rotator|MakeRotfromX (.Normal (Collision|BreakHitResult _outhit))) "0.300000,0.300000,0.300000" true "AutoRelease")))
        (:then_1
          (Effects|SpawnEmitterAttached "/Game/InfinityBladeEffects/Effects/FX_Monsters/FX_Monster_Gruntling/Master/P_BackPack_MuzzleFlash.P_BackPack_MuzzleFlash" (Variables|Default|GetRifle) "Muzzle" (.location _returnvalue) (.rotation _returnvalue) "0.200000,0.200000,0.200000" "KeepWorldPosition" true "AutoRelease")
          (Camera|PlayWorldCameraShake "/Game/Blueprints/BP_RifleFireCameraShake.BP_RifleFireCameraShake_C" (Transformation|GetActorLocation) 0.0 5e+02)
          (Audio|PlaySoundatLocation "/Game/Audio/MS_RifleFire.MS_RifleFire" (Transformation|GetActorLocation) "0, 0, 0" 1.0 1.0 0.0 0 0 0 0))))))

(event Custom|Set%20Strafe%20Movement
  (bind _charactermovement (Variables|Character|GetCharacterMovement))
  ;[0.2135 0.2135 0.2135] Aiming
  (Variables|/Script/Engine.CharacterMovementComponent|SetbOrientRotationToMovement _charactermovement false)
  (Variables|/Script/Engine.CharacterMovementComponent|SetbUseControllerDesiredRotation _charactermovement true))

(event Custom|Set%20Free%20Movement
  (bind _charactermovement (Variables|Character|GetCharacterMovement))
  ;[0.2135 0.2135 0.2135] Aiming
  (Variables|/Script/Engine.CharacterMovementComponent|SetbOrientRotationToMovement _charactermovement true)
  (Variables|/Script/Engine.CharacterMovementComponent|SetbUseControllerDesiredRotation _charactermovement false))

(event Input|EnhancedActionEvents|EnhancedInputActionIA_Move
  (params (ActionValue :type Vector%202D%20Structure) (ElapsedSeconds :type Float%20%28double-precision%29) (TriggeredSeconds :type Float%20%28double-precision%29) (InputAction :type Input%20Action%20Object%20Reference :default "/Game/Input/IA_Move.IA_Move"))
  (bind _returnvalue (Pawn|GetControlRotation :!class /Script/Engine.Pawn))
  (bind _returnvalue_2 (Pawn|GetControlRotation :!class /Script/Engine.Pawn))
  ;[0.2135 0.2135 0.2135] Movment and Camera Look
  (Pawn|Input|AddMovementInput (Math|Vector|GetRightVector (Math|Rotator|MakeRotator (.roll _returnvalue_2) 0.0 (.yaw _returnvalue_2))) (.x ActionValue) false)
  (Pawn|Input|AddMovementInput (Math|Vector|GetForwardVector (Math|Rotator|MakeRotator (.roll _returnvalue) 0.0 (.yaw _returnvalue))) (.y ActionValue) false))

(event Input|EnhancedActionEvents|EnhancedInputActionIA_Look
  (params (ActionValue :type Vector%202D%20Structure) (ElapsedSeconds :type Float%20%28double-precision%29) (TriggeredSeconds :type Float%20%28double-precision%29) (InputAction :type Input%20Action%20Object%20Reference :default "/Game/Input/IA_Look.IA_Look"))
  ;[0.2135 0.2135 0.2135] Movment and Camera Look
  (Pawn|Input|AddControllerYawInput (.x ActionValue))
  (Pawn|Input|AddControllerPitchInput (* (.y ActionValue) -1.0)))

(event Input|EnhancedActionEvents|EnhancedInputActionIA_EquipeRifle
  (params (ActionValue :type Boolean) (ElapsedSeconds :type Float%20%28double-precision%29) (TriggeredSeconds :type Float%20%28double-precision%29) (InputAction :type Input%20Action%20Object%20Reference :default "/Game/Input/IA_EquipeRifle.IA_EquipeRifle"))
  ;[0.2135 0.2135 0.2135] Equip and Unequip Rifle
  (:Started
    (if (not (Variables|Default|GetRifle%20Equipped))
      (Variables|Default|SetRifle%20Equipped true)
      (Utilities|FlowControl|Delay 0.5)
      (Rendering|SetVisibility (Variables|Default|GetRifle) true false)
      (else
        (Variables|Default|SetRifle%20Equipped false)
        (Utilities|FlowControl|Delay 0.5)
        (Rendering|SetVisibility (Variables|Default|GetRifle) false false)))))

(event Input|EnhancedActionEvents|EnhancedInputActionIA_Aim
  (params (ActionValue :type Boolean) (ElapsedSeconds :type Float%20%28double-precision%29) (TriggeredSeconds :type Float%20%28double-precision%29) (InputAction :type Input%20Action%20Object%20Reference :default "/Game/Input/IA_Aim.IA_Aim"))
  (bind _springarm (Variables|Default|GetSpringArm))
  ;[0.2135 0.2135 0.2135] Aiming
  (:Started
    (Variables|Default|SetIs%20Aiming true)
    (CallFunction|SetStrafeMovement)
    (bind _arm_lenghth (Timeline|Aim Play)
      (:Update
        (Variables|/Script/Engine.SpringArmComponent|SetTargetArmLength (Variables|Default|GetSpringArm) (Math|Float|Lerp 3e+02 1.5e+02 _arm_lenghth))
        (Variables|/Script/Engine.SpringArmComponent|SetSocketOffset _springarm (Math|Vector|MakeVector (.x (Variables|/Script/Engine.SpringArmComponent|GetSocketOffset _springarm)) (Math|Float|Lerp 25.0 5e+01 _arm_lenghth) (Math|Float|Lerp 0.0 25.0 _arm_lenghth))))))
  (:Completed
    (Variables|Default|SetIs%20Aiming false)
    (CallFunction|SetFreeMovement)
    (Timeline|Aim Reverse)))

(event Input|EnhancedActionEvents|EnhancedInputActionIA_Fire
  (params (ActionValue :type Boolean) (ElapsedSeconds :type Float%20%28double-precision%29) (TriggeredSeconds :type Float%20%28double-precision%29) (InputAction :type Input%20Action%20Object%20Reference :default "/Game/Input/IA_Fire.IA_Fire"))
  (:Started
    (if (Variables|Default|GetRifle%20Equipped)
      (bind _returnvalue (Utilities|Time|SetTimerbyEvent (delegate Custom|Fire%20Rifle) 0.1 true))))
  (:Completed
    (Utilities|Time|ClearandInvalidateTimerbyHandle _returnvalue)))

(event EventBeginPlay
  ;[0.2135 0.2135 0.2135] Add Input
  (Input|AddMappingContext (PlayerController|LocalPlayerSubsystems|GetEnhancedInputLocalPlayerSubsystem (Game|GetPlayerController 0)) "/Game/Input/IMC_PlayerInput.IMC_PlayerInput" 0 "(bIgnoreAllPressedKeysUntilRelease=True,bForceImmediately=False,bNotifyUserSettings=False)")
  (bind _returnvalue (UserInterface|CreateWidget "/Game/UI/WB_HUD.WB_HUD_C"))
  (UserInterface|Viewport|AddtoViewport _returnvalue 0))

(fn ConstructionScript)